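; BP_Canon is a cannon actor that fires projectiles automatically on a repeating cycle from BeginPlay.
; After a FireRate delay, it spawns BP_Projectile at the Arrow component's world transform and plays a firing timeline from the start.
; The timeline animates the Cannon component's relative Y location, and its Start Cannon Fired event track loops execution back to the delay.
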(event EventBeginPlay
  (Utilities|FlowControl|Delay (Variables|Default|GetFire%20rate) :!label _label)
  (CallFunction|SpawnProjectile)
  (bind _shoot_cannon_position (Timeline|Canon_fire_timeline PlayFromStart)
    (:Update
      (CallFunction|FireCannon _shoot_cannon_position))
    (:Start_cannon_fired
      (goto _label))))

(event Collision|EventActorBeginOverlap
  (params (OtherActor :type Actor%20Object%20Reference)))

(event EventTick
  (params (DeltaSeconds :type Float%20%28single-precision%29)))

(fn ConstructionScript)

(fn SpawnProjectile
  (bind _arrow (Variables|Default|GetArrow))
  (Game|SpawnActorfromClass "/Game/Blueprint_Classes/BP_Projectile.BP_Projectile_C" (Math|Transform|MakeTransform (Transformation|GetWorldLocation _arrow) (Transformation|GetWorldRotation _arrow) "1,1,1") "Undefined" 0 0))

(fn FireCannon
  (params (NewLocation_Y :type Float%20%28single-precision%29))
  (Transformation|SetRelativeLocation (Variables|Default|Getcannon) (Math|Vector|MakeVector 0.0 NewLocation_Y 0.0) false false))