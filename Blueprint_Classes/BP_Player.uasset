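; BP_Player is the player-controlled actor, moved by rolling its static mesh with physics torque.
; The forward/backward and left/right input axes, scaled by AccelerationMultiplier, apply torque around the X and Y axes respectively.
; Taking any damage runs Reset level, which fades the camera to near-black, waits for the fade to finish, then reopens the current level.
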(event EventBeginPlay)

(event Collision|EventActorBeginOverlap
  (params (OtherActor :type Actor%20Object%20Reference)))

(event EventTick
  (params (DeltaSeconds :type Float%20%28single-precision%29)))

(event Game|Damage|EventAnyDamage
  (params (Damage :type Float%20%28single-precision%29) (DamageType :type Damage%20Type%20Object%20Reference) (InstigatedBy :type Controller%20Object%20Reference) (DamageCauser :type Actor%20Object%20Reference))
  (Utilities|ResetLevel))

(event Input|AxisEvents|InputAxisforward_backward
  (params (AxisValue :type Float%20%28single-precision%29))
  (Class|PrimitiveComponent|AddTorqueinRadians (Variables|Default|GetStaticMesh) (Math|Vector|MakeVector (* AxisValue (Variables|Default|GetAccelerationMultiplier)) 0.0 0.0) "None" false))

(event Input|AxisEvents|InputAxisleft_right
  (params (AxisValue :type Float%20%28single-precision%29))
  (Class|PrimitiveComponent|AddTorqueinRadians (Variables|Default|GetStaticMesh) (Math|Vector|MakeVector 0.0 (* AxisValue (Variables|Default|GetAccelerationMultiplier)) 0.0) "None" false))

(fn ConstructionScript)