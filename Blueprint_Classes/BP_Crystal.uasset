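; BP_Crystal is a collectible crystal actor that animates into the player on overlap, then destroys itself.
; On overlap, an IsPlayer check gates storing its location, scale and point light intensity, then plays a timeline.
; Each update lerps the crystal toward the player pawn's current location, shrinks it to zero scale and fades the light, using separate curves for motion and light.
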(event EventBeginPlay)

(event Collision|EventActorBeginOverlap
  (params (OtherActor :type Actor%20Object%20Reference))
  (Utilities|IsPlayer OtherActor
    (:Is%20player
      (CallFunction|StoreStartingValues)
      (bind (_direction _collection_timeline _light_intensity) (Timeline|Timeline_0 Play)
        (:Update
          (CallFunction|MovetoPlay _collection_timeline)
          (CallFunction|ScaleFunctions _collection_timeline)
          (CallFunction|AdjustLight _light_intensity))
        (:Finished
          (Actor|DestroyActor))))))

(event EventTick
  (params (DeltaSeconds :type Float%20%28single-precision%29)))

(fn ConstructionScript)

(fn MovetoPlay
  (params (Alpha :type Float%20%28single-precision%29))
  (Transformation|SetActorLocation (Math|Vector|Lerp(Vector) (Variables|Default|GetLerp_start_location) (Transformation|GetActorLocation (Game|Player|GetPlayerPawn 0)) Alpha) false false))

(fn StoreStartingValues
  (Variables|Default|SetLerp_start_location (Transformation|GetActorLocation))
  (Variables|Default|SetOriginal%20scale (Transformation|GetActorScale3D))
  (Variables|Default|SetStart%20light%20intensity (Variables|/Script/Engine.LightComponentBase|GetIntensity (Variables|Default|GetPointLight))))

(fn ScaleFunctions
  (params (Alpha :type Float%20%28single-precision%29))
  (Transformation|SetActorScale3D (Math|Vector|Lerp(Vector) (Variables|Default|GetOriginal%20scale) "0, 0, 0" Alpha)))

(fn AdjustLight
  (params (Alpha :type Float%20%28single-precision%29))
  (Rendering|Components|Light|SetIntensity (Variables|Default|GetPointLight) (Math|Float|Lerp (Variables|Default|GetStart%20light%20intensity) 0.0 Alpha)))